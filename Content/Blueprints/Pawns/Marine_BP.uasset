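; Player marine pawn for a twin-stick shooter, with world-axis movement, health, a kill counter and a HUD created at BeginPlay.
; Each Tick sets control rotation from thumbstick direction or smoothed mouse velocity, depending on the last key pressed, with deadzones on both.
; Firing runs a looping timer of damaging line traces from the muzzle socket, with particles, sound and debug lines.
; Death stops firing and calls OnDeath once.
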(event EventTick
  (params (DeltaSeconds :type Float%20%28single-precision%29))
  (CallFunction|UpdatePlayerAim))

(event EventBeginPlay
  (bind _returnvalue (UserInterface|CreateWidget "/Game/UI/W_PlayerHUD.W_PlayerHUD_C" 0 self))
  (UserInterface|Viewport|AddtoViewport _returnvalue 0))

(event Game|Damage|EventAnyDamage
  (params (Damage :type Float%20%28single-precision%29) (DamageType :type Damage%20Type%20Object%20Reference) (InstigatedBy :type Controller%20Object%20Reference) (DamageCauser :type Actor%20Object%20Reference))
  (bind _health (CallFunction|DecreaseHealth Damage))
  (if (<= _health 0.0)
    (Variables|Default|SetDead true)
    (Utilities|FlowControl|DoOnce false
      (:Completed
        (CallFunction|StopFiringWeapon)
        (Default|CallOnDeath)))))

(event Input|ActionEvents|InputActionFireWeapon
  (params (Key :type Key%20Structure))
  (:Pressed
    (CallFunction|StartFiringWeapon)
    (CallFunction|WeaponTrace)
    (Utilities|Time|SetTimerbyFunctionName 0 "Weapon Trace" (Variables|Default|GetWeapon%20Fire%20Rate) true))
  (:Released
    (CallFunction|StopFiringWeapon)))

(event Input|AxisEvents|InputAxisMoveForward
  (params (AxisValue :type Float%20%28single-precision%29))
  (if (CallFunction|IsAlive)
    (Pawn|Input|AddMovementInput "1.000000, 0, 0" AxisValue false)))

(event Input|AxisEvents|InputAxisMoveRight
  (params (AxisValue :type Float%20%28single-precision%29))
  (if (CallFunction|IsAlive)
    (Pawn|Input|AddMovementInput "0,1.000000, 0" AxisValue false)))

(event Input|KeyboardEvents|AnyKey
  (params (Key :type Key%20Structure))
  (:Pressed
    (Variables|Default|SetGamepad%20Active (Class|KismetInputLibrary|KeyIsGamepadKey Key))))

(fn ConstructionScript)

(fn UpdatePlayerAim
  (if (CallFunction|IsAlive)
    (if (Variables|Default|GetGamepad%20Active)
      (Thumbstick|UpdateThumbstickAim)
      (else
        (MouseInput|UpdateMouseAim)))))

(fn IsThumbstickAboveDeadzone
  (return (> (Math|Vector2D|Vector2DLength (Math|Vector2D|MakeVector2D (Input|AxisValues|GetThumbstickAimRight) (Input|AxisValues|GetThumbstickAimUp))) (Variables|Default|GetThumbstick%20Deadzone))))

(fn GetMouseVelocity
  (bind _returnvalue (Game|GetPlayerController 0))
  (bind (_deltax _deltay) (Class|PlayerController|GetInputMouseDelta _returnvalue))
  (return (/ (Math|Vector2D|MakeVector2D _deltax _deltay) (Utilities|Time|GetWorldDeltaSeconds))))

(fn IsMouseAboveDeadzone
  (bind _returnvalue (MouseInput|GetMouseVelocity))
  (return (> (Math|Vector2D|Vector2DLength (Math|Vector2D|MakeVector2D (.x _returnvalue) (.y _returnvalue))) (Variables|Default|GetMouse%20Deadzone))))

(fn UpdateMouseAim
  (if (MouseInput|IsMouseAboveDeadzone)
    (Pawn|SetControlRotation (Game|GetPlayerController 0) (MouseInput|GetMouseAimDirection))))

(fn GetMouseAimDirection
  (bind _returnvalue (MouseInput|GetMouseVelocity))
  (return (Math|Interpolation|RInterpTo (Pawn|GetControlRotation (Game|GetPlayerController 0) :!class /Script/Engine.Controller) (Math|Rotator|MakeRotator 0.0 0.0 (Class|KismetMathLibrary|DegAtan2 (.x _returnvalue) (.y _returnvalue))) (Utilities|Time|GetWorldDeltaSeconds) (Variables|Default|GetMouse%20Smoothing%20Strength))))

(fn UpdateThumbstickAim
  (if (Thumbstick|IsThumbstickAboveDeadzone)
    (Pawn|SetControlRotation (Game|GetPlayerController 0) (Thumbstick|GetThumstickAimDirection))))

(fn GetThumstickAimDirection
  (return (Math|Rotator|MakeRotator 0.0 0.0 (Class|KismetMathLibrary|DegAtan2 (Input|AxisValues|GetThumbstickAimRight) (Input|AxisValues|GetThumbstickAimUp)))))

(fn StartFiringWeapon
  (if (CallFunction|IsAlive)
    (Components|Activation|Activate (Variables|Default|GetP_AssaultRifle_MF) false)
    (bind _returnvalue (Audio|SpawnSound2D "/Game/Sounds/Weapon_AssaultRifle/Stereo/RifleFiring_Cue.RifleFiring_Cue" 1.0 1.0 0.0 0))
    (Variables|Default|SetWeapon%20Fire%20Sound _returnvalue)
    (Variables|Default|SetIsFiring true)))

(fn StopFiringWeapon
  (if (Variables|Default|GetIsFiring)
    (Components|Activation|Deactivate (Variables|Default|GetP_AssaultRifle_MF))
    (Audio|Components|Audio|Stop (Variables|Default|GetWeapon%20Fire%20Sound))
    (Utilities|Time|ClearTimerbyFunctionName 0 "Weapon Trace")
    (if (CallFunction|IsAlive)
      (Audio|SpawnSound2D "/Game/Sounds/Weapon_AssaultRifle/Stereo/RifleFireEnd_Cue.RifleFireEnd_Cue" 1.0 1.0 0.0 0)
      (Variables|Default|SetIsFiring false))))

(fn DecreaseHealth
  (params (Damage%20Amount :type Float%20%28single-precision%29))
  (bind _output_get (Variables|Default|SetHealth (Math|Float|Clamp(Float) (- (Variables|Default|GetHealth) Damage%20Amount) 0.0 1e+02)))
  (return _output_get))

(fn IsAlive
  (return (not (Variables|Default|GetDead))))

(fn WeaponTrace
  (bind _outhit (Collision|LineTraceByChannel (CallFunction|GetWeaponTraceStartLocation) (CallFunction|GetWeaponTraceEndLocation) "TraceTypeQuery1" false 0 "ForDuration"))
  (if (.bBlockingHit (Collision|BreakHitResult _outhit))
    (Game|Damage|ApplyDamage (.HitActor (Collision|BreakHitResult _outhit)) (Variables|Default|GetDamage%20Per%20Shot) 0 0)))

(fn GetWeaponTraceStartLocation
  (return (Transformation|GetSocketLocation (Variables|Default|GetRifle) "MuzzleFlash")))

(fn GetWeaponTraceEndLocation
  (return (+ (CallFunction|GetWeaponTraceStartLocation) (* (Math|Vector|GetForwardVector (Pawn|GetControlRotation :!class /Script/Engine.Pawn)) (Variables|Default|GetWeapon%20Rage)))))

(fn IncreaseKills
  (Math|Integer|IncrementInt (Variables|Default|GetKills)))